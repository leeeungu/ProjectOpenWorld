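; Test player Blueprint with debug hotkeys for exercising Pal jobs and save/load.
; Keys find a PinkCat Pal in the world and push mining, item transport or attack work into its job component; only attack also calls StartWorking.
; Numpad keys save the world and load the player save slot.
; Disconnected leftover graphs cover spawning and storing a Pal, building work and base camp work commands.
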(event EventBeginPlay
  (|CallParentFunction))

(event Input|KeyboardEvents|DebugKeyNumPadEight
  (params (Key :type Key%20Structure :default "None") (ActionValue :type Input%20Action%20Value%20Structure))
  (:Pressed
    (Class|BaseGameInstance|LoadfromSlot self "PlayerSave")))

(event Input|KeyboardEvents|DebugKey1
  (params (Key :type Key%20Structure :default "None") (ActionValue :type Input%20Action%20Value%20Structure)))

(event Input|KeyboardEvents|DebugKey2
  (params (Key :type Key%20Structure :default "None") (ActionValue :type Input%20Action%20Value%20Structure))
  (:Pressed
    (Utilities|FlowControl|Sequence
      (:then_0
        (bind _returnvalue (Actor|GetActorOfClass "/Game/Pal/Model/Monster/PinkCat/Bp_PinkCat_Pal.Bp_PinkCat_Pal_C")))
      (:then_1
        (bind _returnvalue_2 (Actor|GetActorOfClass "/Script/ProjectOpenWorld.PalHarvestActor"))
        (Class|PalJobComponent|TryPushJob (Class|PalBaseCreature|GetJobComponent _returnvalue) (Class|PalCommandFunctionLibrary|WorkMining self _returnvalue_2))))))

(event Input|KeyboardEvents|DebugKey3
  (params (Key :type Key%20Structure :default "None") (ActionValue :type Input%20Action%20Value%20Structure))
  (bind _self self)
  (:Pressed
    (Utilities|FlowControl|Sequence
      (:then_0
        (bind _returnvalue (Actor|GetActorOfClass "/Game/Pal/Model/Monster/PinkCat/Bp_PinkCat_Pal.Bp_PinkCat_Pal_C")))
      (:then_1
        (bind _returnvalue_2 (Actor|GetActorOfClass "/Script/ProjectOpenWorld.ItemActor"))
        (Utilities|IsValid _returnvalue_2
          (:Is%20Valid
            (Class|PalJobComponent|TryPushJob (Class|PalBaseCreature|GetJobComponent _returnvalue) (Class|PalCommandFunctionLibrary|WorkTransport _self _returnvalue_2 _self))))))))

(event Input|KeyboardEvents|DebugKey4
  (params (Key :type Key%20Structure :default "None") (ActionValue :type Input%20Action%20Value%20Structure))
  (:Pressed
    (Utilities|FlowControl|Sequence
      (:then_0
        (bind _returnvalue (Actor|GetActorOfClass "/Game/Pal/Model/Monster/PinkCat/Bp_PinkCat_Pal.Bp_PinkCat_Pal_C")))
      (:then_1
        (bind _returnvalue_2 (Actor|GetActorOfClass "/Game/Pal/Model/Monster/PinkCat/Bp_PinkCat_Monster.Bp_PinkCat_Monster_C"))
        (Utilities|IsValid _returnvalue_2
          (:Is%20Valid
            (Class|PalJobComponent|TryPushJob (Class|PalBaseCreature|GetJobComponent _returnvalue) (Class|PalCommandFunctionLibrary|WorkAttack self _returnvalue_2))
            (Class|PalJobComponent|StartWorking (Class|PalBaseCreature|GetJobComponent _returnvalue))))))))

(event Input|KeyboardEvents|DebugKey5
  (params (Key :type Key%20Structure :default "None") (ActionValue :type Input%20Action%20Value%20Structure)))

(event Input|KeyboardEvents|DebugKeyNumPadSeven
  (params (Key :type Key%20Structure :default "None") (ActionValue :type Input%20Action%20Value%20Structure))
  (:Pressed
    (Class|BaseGameInstance|SaveWorld)))

(fn ConstructionScript
  (|CallParentFunction))