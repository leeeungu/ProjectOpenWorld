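; Test player Blueprint with numpad debug keys for exercising boss combat, base camp storage and foliage removal.
; On BeginPlay it caches Anubis boss actors, which keys use to trigger a skill attack on the player and damage calls either way.
; Other keys toggle StartResource/StopResource, store Pals in the targeted base camp, or sphere-trace to delete nearby foliage instances.
; Unwired command, battle-state and line-trace experiments remain in the graph.
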(event EventBeginPlay
  (|CallParentFunction)
  (bind _outactors (Actor|GetAllActorsOfClass "/Game/Pal/Model/Monster/Anubis/Boss/Bp_Anubis_Boss.Bp_Anubis_Boss_C"))
  (Variables|Default|SetOut%20Actors _outactors))

(event Input|KeyboardEvents|DebugKeyNumPadSix
  (params (Key :type Key%20Structure :default "None") (ActionValue :type Input%20Action%20Value%20Structure))
  (:Pressed
    (Utilities|FlowControl|FlipFlop
      (:A
        (Class|ResourceInterface|StartResource))
      (:B
        (Class|ResourceInterface|StopResource)))))

(event Input|KeyboardEvents|DebugKeyNumPadSeven
  (params (Key :type Key%20Structure :default "None") (ActionValue :type Input%20Action%20Value%20Structure))
  (bind _interactioncomponent (Variables|Default|GetInteractionComponent))
  (bind _returnvalue (Class|InteractionComponent|GetTargetActor _interactioncomponent))
  (:Pressed
    (Utilities|IsValid _returnvalue
      (:Is%20Valid
        (bind _aspal_base_camp (Utilities|Casting|CastToPalBaseCamp _returnvalue))
        (Class|PalStorageComponent|StorePal (Variables|/Script/ProjectOpenWorld.PalBaseCamp|GetPalStore _aspal_base_camp) (Utilities|Struct|MakePalStoreInventoryData "/Game/Pal/Model/Monster/Anubis/Temp/Bp_Anubis_Pal.Bp_Anubis_Pal_C" false))))))

(event Input|KeyboardEvents|DebugKeyNumPadFour
  (params (Key :type Key%20Structure :default "None") (ActionValue :type Input%20Action%20Value%20Structure))
  (bind _returnvalue (Transformation|GetActorLocation))
  (:Pressed
    (bind _outhits (Collision|MultiSphereTraceByChannel _returnvalue _returnvalue 1.2e+03 "TraceTypeQuery1" false 0 "None"))
    (for _array_element _outhits
      (bind _asfoliage_instanced_static_mesh_component (Utilities|Casting|CastToFoliageInstancedStaticMeshComponent (.HitComponent (Collision|BreakHitResult _array_element))))
      (Development|PrintString (Utilities|GetDisplayName _asfoliage_instanced_static_mesh_component))
      (Class|InstancedStaticMeshComponent|RemoveInstances _asfoliage_instanced_static_mesh_component (Class|InstancedStaticMeshComponent|GetInstancesOverlappingSphere _asfoliage_instanced_static_mesh_component (.Location (Collision|BreakHitResult _array_element)) 1e+01 true)))))

(event Input|KeyboardEvents|DebugKeyNumPadTwo
  (params (Key :type Key%20Structure :default "None") (ActionValue :type Input%20Action%20Value%20Structure))
  (:Pressed
    (Class|AttackInterface|DamagedCharacter (Utilities|Array|Get(acopy) (Variables|Default|GetOut%20Actors)) self)))

(event Input|KeyboardEvents|DebugKeyNumPadOne
  (params (Key :type Key%20Structure :default "None") (ActionValue :type Input%20Action%20Value%20Structure))
  (bind _out_actors (Variables|Default|GetOut%20Actors))
  (bind _output (Utilities|Array|Get(acopy) _out_actors))
  (bind _attackcomponent (Variables|/Script/ProjectOpenWorld.BaseMonster|GetAttackComponent _output))
  (:Pressed
    (Utilities|IsValid _output
      (:Is%20Valid
        (Class|PalAttackComponent|SetAttackData _attackcomponent "Skill01")
        (Class|PalAttackComponent|SetAttackTarget _attackcomponent self)
        (Class|PalAttackComponent|StartAttack _attackcomponent)))))

(event Input|KeyboardEvents|DebugKeyNumPadThree
  (params (Key :type Key%20Structure :default "None") (ActionValue :type Input%20Action%20Value%20Structure))
  (:Pressed
    (bind _returnvalue (Class|AttackInterface|DamagedCharacter self (Utilities|Array|Get(acopy) (Variables|Default|GetOut%20Actors))))
    (Development|PrintString (Utilities|String|ToString(Boolean) _returnvalue))))

(event Input|KeyboardEvents|DebugKeyNumPadFive
  (params (Key :type Key%20Structure :default "None") (ActionValue :type Input%20Action%20Value%20Structure))
  (bind _interactioncomponent (Variables|Default|GetInteractionComponent))
  (bind _returnvalue (Class|InteractionComponent|GetTargetActor _interactioncomponent))
  (:Pressed
    (Utilities|IsValid _returnvalue
      (:Is%20Valid
        (bind _aspal_base_camp (Utilities|Casting|CastToPalBaseCamp _returnvalue))
        (Class|PalStorageComponent|StorePal (Variables|/Script/ProjectOpenWorld.PalBaseCamp|GetPalStore _aspal_base_camp) (Utilities|Struct|MakePalStoreInventoryData "/Game/Pal/Model/Monster/PinkCat/Bp_PinkCat_Pal.Bp_PinkCat_Pal_C" false))))))

(fn ConstructionScript
  (|CallParentFunction))