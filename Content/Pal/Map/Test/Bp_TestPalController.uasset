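; Test controller Blueprint for Pal, kept in the map test folder, that seeds an inventory with starter items.
; On BeginPlay it runs the parent logic, then creates base items for a sword, steel pickaxe and axe, and a stack of wood.
; Each item is added to the InventoryComponent as soon as it is created.
; The construction script only calls its parent.
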(event `self.ReceiveBeginPlay`
  (bind _inventorycomponent (`self.InventoryComponent`))
  (`parent.ReceiveBeginPlay`)
  (bind _returnvalue (`ItemFunctionLibrary.CreateBaseItem` "Sword" 1 self "/Script/ProjectOpenWorld.BaseItem"))
  (`InventoryComponent.AddItem` (`self.InventoryComponent`) _returnvalue)
  (bind _returnvalue_2 (`ItemFunctionLibrary.CreateBaseItem` "Pickaxe_Steal" 1 self "/Script/ProjectOpenWorld.BaseItem"))
  (`InventoryComponent.AddItem` _inventorycomponent _returnvalue_2)
  (bind _returnvalue_3 (`ItemFunctionLibrary.CreateBaseItem` "Axe_Steal" 1 self "/Script/ProjectOpenWorld.BaseItem"))
  (`InventoryComponent.AddItem` _inventorycomponent _returnvalue_3)
  (bind _returnvalue_4 (`ItemFunctionLibrary.CreateBaseItem` "Wood" 100 self "/Script/ProjectOpenWorld.BaseItem"))
  (`InventoryComponent.AddItem` _inventorycomponent _returnvalue_4))

(fn `UserConstructionScript`
  (`parent.UserConstructionScript`))