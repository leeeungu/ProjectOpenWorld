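; Anubis soldier monster Blueprint that reacts to players entering its trigger box.
; When a BasePlayer overlaps the Box, the mesh plays the Attack03 montage; when the player leaves, the montage stops with a short blend-out.
; The construction script runs the parent's, then destroys the inherited HP widget component, so no health bar is shown.
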(event `self.Box.OnComponentBeginOverlap`
  (params (OverlappedComponent :type "PrimitiveComponent Object Reference") (OtherActor :type "Actor Object Reference") (OtherComp :type "PrimitiveComponent Object Reference") (OtherBodyIndex :type Integer) (bFromSweep :type Boolean) (SweepResult :type "HitResult Structure (by ref)"))
  (cast `BasePlayer` OtherActor)
  (`|PlayMontage` (`self.Mesh`) "/Game/Pal/Model/Monster/Anubis/Montage/SoilderAttack/AS_Anubis_Attack03_Montage.AS_Anubis_Attack03_Montage"))

(event `self.Box.OnComponentEndOverlap`
  (params (OverlappedComponent :type "PrimitiveComponent Object Reference") (OtherActor :type "Actor Object Reference") (OtherComp :type "PrimitiveComponent Object Reference") (OtherBodyIndex :type Integer))
  (cast `BasePlayer` OtherActor)
  (`AnimInstance.Montage_Stop` (`SkeletalMeshComponent.GetAnimInstance` (`self.Mesh`)) 0.25 null))

(fn `UserConstructionScript`
  (`parent.UserConstructionScript`)
  (`ActorComponent.K2_DestroyComponent` (`self.HpWidgetComponent`)))