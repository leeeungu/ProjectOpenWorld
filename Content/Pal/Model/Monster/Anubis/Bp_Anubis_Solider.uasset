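; Anubis soldier monster Blueprint that acts as a stationary attacker, with character movement disabled on BeginPlay.
; A Box overlap serves as its detection zone, reacting only to BasePlayer actors.
; Entering the box passes that player to the AttackComponent as the target on the Default attack slot, and leaving it ends the attack.
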(event `self.Box.OnComponentBeginOverlap`
  (params (OverlappedComponent :type "PrimitiveComponent Object Reference") (OtherActor :type "Actor Object Reference") (OtherComp :type "PrimitiveComponent Object Reference") (OtherBodyIndex :type Integer) (bFromSweep :type Boolean) (SweepResult :type "HitResult Structure (by ref)"))
  (bind _asbase_player (cast `BasePlayer` OtherActor))
  (`PalAttackComponent.SetAttackData` (`self.AttackComponent`) (make `PalAttackData` _asbase_player "Default")))

(event `self.ReceiveBeginPlay`
  (`CharacterMovementComponent.DisableMovement` (`self.CharacterMovement`)))

(event `self.Box.OnComponentEndOverlap`
  (params (OverlappedComponent :type "PrimitiveComponent Object Reference") (OtherActor :type "Actor Object Reference") (OtherComp :type "PrimitiveComponent Object Reference") (OtherBodyIndex :type Integer))
  (cast `BasePlayer` OtherActor)
  (`PalAttackComponent.EndAttack` (`self.AttackComponent`)))

(fn `UserConstructionScript`
  (`parent.UserConstructionScript`))