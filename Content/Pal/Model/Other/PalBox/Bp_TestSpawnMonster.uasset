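; Test actor in the PalBox folder that spawns CaptainPenguin monsters and also serves as a move command source.
; BeginPlay starts a looping timer, and SpawnMonster force-spawns a penguin slightly above a random reachable navmesh point around the actor.
; Its command overrides return a move-to-actor command targeting itself that never reports finished.
; An array-driven spawn loop and a random-location move command are left unconnected.
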(event `self.ReceiveBeginPlay`
  (`KismetSystemLibrary.K2_SetTimerDelegate` (`|CreateDelegate` :!event `Spawn Monster`) 5.0 true))

(event `Spawn Monster`
  (`|SpawnActorFromClass` "/Game/Pal/Model/Monster/CaptainPenguin/Bp_CaptainPenguin_Monster.Bp_CaptainPenguin_Monster_C" (`KismetMathLibrary.MakeTransform` (+ (`NavigationSystemV1.K2_GetRandomReachablePointInRadius` (`self.K2_GetActorLocation`) 1200.0 null null) (0.0 0.0 100.0))) "AdjustIfPossibleButAlwaysSpawn" "MultiplyWithRoot" null null))

(fn `GetCommand`
  (returns (ReturnValue :type "PalCommand Structure"))
  (return (`PalCommandFunctionLibrary.CommandMoveToActor` self self)))

(fn `GetCommandKind`
  (returns (ReturnValue :type "EPalCommandKind Enum"))
  (return "Move"))

(fn `GetSubCommandType`
  (returns (ReturnValue :type Byte))
  (return (enumliteral `ESubMoveType` "Actor")))

(fn `IsCommandFinished`
  (returns (ReturnValue :type Boolean))
  (return false))

(fn `UserConstructionScript`)