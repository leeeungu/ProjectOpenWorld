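; Test spawner actor in the PalBox model folder that spawns Bp_TestResource actors and doubles as a move-command source.
; BeginPlay starts a looping six-second timer, while SpawnMonster places a resource at a random reachable point around the actor, adjusting for collisions.
; Its command overrides issue an actor-targeted move toward itself that never reports as finished.
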(event `self.ReceiveBeginPlay`
  (`KismetSystemLibrary.K2_SetTimerDelegate` (`|CreateDelegate` :!event `Spawn Monster`) 6.0 true))

(event `Spawn Monster`
  (`|SpawnActorFromClass` :`Class` "/Game/Pal/Model/Other/PalBox/Bp_TestResource.Bp_TestResource_C" :`SpawnTransform` (`KismetMathLibrary.MakeTransform` (`NavigationSystemV1.K2_GetRandomReachablePointInRadius` (`self.K2_GetActorLocation`) 1200.0 null null)) :`CollisionHandlingOverride` "AdjustIfPossibleButAlwaysSpawn" :`TransformScaleMethod` "MultiplyWithRoot" :`Instigator` null))

(fn `GetCommand`
  (returns (ReturnValue :type "PalCommand Structure"))
  (return (`PalCommandFunctionLibrary.CommandMoveToActor` self self)))

(fn `GetCommandKind`
  (returns (ReturnValue :type "EPalCommandKind Enum"))
  (return "Move"))

(fn `GetSubCommandType`
  (returns (ReturnValue :type Byte))
  (return (enumliteral `ESubMoveType` "Actor")))

(fn `IsCommandFinished`
  (returns (ReturnValue :type Boolean))
  (return false))

(fn `UserConstructionScript`)