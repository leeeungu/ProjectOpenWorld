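; Test storage Blueprint under PalBox that offers a transport work command with itself as the destination.
; StoreItem caches an ItemActor found in the world, and GetCommand passes it as the transport target, with the storage as both instigator and destination.
; The command reports Work kind with a Transport subtype and never finishes.
; The logic that prints the stored item and destroys an actor is disconnected and never runs.
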(event `self.ReceiveBeginPlay`
  (`parent.ReceiveBeginPlay`))

(event `StoreItem`
  (bind _returnvalue (`GameplayStatics.GetActorOfClass` "/Script/ProjectOpenWorld.ItemActor"))
  (set `self.NewVar_0` _returnvalue))

(fn `GetCommand`
  (returns (ReturnValue :type "PalCommand Structure"))
  (return (`PalCommandFunctionLibrary.CommandTransport` self (`self.NewVar_0`) self)))

(fn `GetCommandKind`
  (returns (ReturnValue :type "EPalCommandKind Enum"))
  (return "Work"))

(fn `GetSubCommandType`
  (returns (ReturnValue :type Byte))
  (return (enumliteral `ESubWorkType` "Transport")))

(fn `IsCommandFinished`
  (returns (ReturnValue :type Boolean))
  (return false))

(fn `UserConstructionScript`)