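; Test Pal Sphere blueprint that offers itself as a transport work command.
; On BeginPlay it finds a Bp_TestSpawnMonster actor and stores it as the destination.
; GetCommand builds a Transport command with itself as instigator and target and that actor as destination, reported as Work kind with Transport subtype.
; IsCommandFinished always returns false, so the command never reports completion.
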(event `self.ReceiveBeginPlay`
  (bind _returnvalue (`GameplayStatics.GetActorOfClass` "/Game/Pal/Model/Other/PalBox/Bp_TestSpawnMonster.Bp_TestSpawnMonster_C"))
  (set `self.NewVar` _returnvalue))

(fn `GetCommand`
  (returns (ReturnValue :type "PalCommand Structure"))
  (return (`PalCommandFunctionLibrary.CommandTransport` self self (`self.NewVar`))))

(fn `GetCommandKind`
  (returns (ReturnValue :type "EPalCommandKind Enum"))
  (return "Work"))

(fn `GetSubCommandType`
  (returns (ReturnValue :type Byte))
  (return (enumliteral `ESubWorkType` "Transport")))

(fn `IsCommandFinished`
  (returns (ReturnValue :type Boolean))
  (return false))

(fn `UserConstructionScript`)