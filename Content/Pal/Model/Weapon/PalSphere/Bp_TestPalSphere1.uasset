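; Test Pal Sphere Blueprint that presents itself as a source of a transport work command.
; Its command getters report the Work kind with a Transport subtype and build a transport command using itself as instigator and target actor, with TargetTransport as the destination.
; The finished check always returns true, and the construction script is empty.
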(fn `GetCommand`
  (returns (ReturnValue :type "PalCommand Structure"))
  (return (`PalCommandFunctionLibrary.CommandTransport` self self (`self.TargetTransport`))))

(fn `GetCommandKind`
  (returns (ReturnValue :type "EPalCommandKind Enum"))
  (return "Work"))

(fn `GetSubCommandType`
  (returns (ReturnValue :type Byte))
  (return (enumliteral `ESubWorkType` "Transport")))

(fn `IsCommandFinished`
  (returns (ReturnValue :type Boolean))
  (return true))

(fn `UserConstructionScript`)