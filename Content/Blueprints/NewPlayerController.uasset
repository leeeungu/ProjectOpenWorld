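; Player controller for building placement, showing a preview cube with an overlay material where the camera aims.
; Each tick a camera line trace and a sphere trace position the preview and find the target actor.
; FindSockets caches that actor's socket locations, and the preview snaps to one near the impact point.
; Debug keys rotate the preview and spawn a Bp_Building with its mesh and transform, then reset the preview's rotation.
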(event EventTick
  (params (DeltaSeconds :type Float%20%28single-precision%29))
  (bind _returnvalue (Game|GetPlayerCameraManager 0))
  (bind _returnvalue_2 (Pawn|GetControlledPawn))
  (bind _buildingmesh (Variables|Default|GetBuildingMesh))
  (bind _returnvalue_3 (Camera|GetCameraLocation _returnvalue))
  (bind _array (Utilities|Array|MakeArray _returnvalue_2 _buildingmesh))
  (bind (_outhit _returnvalue_4) (Collision|LineTraceForObjects _returnvalue_3 (+ _returnvalue_3 (* (Math|Vector|GetForwardVector (Camera|GetCameraRotation _returnvalue)) 1.2e+03)) (Utilities|Array|MakeArray "ObjectTypeQuery1" "ObjectTypeQuery2" "ObjectTypeQuery4") true _array "None"))
  (if _returnvalue_4
    (bind (_outhit_2 _returnvalue_5) (Collision|SphereTraceForObjects (.ImpactPoint (Collision|BreakHitResult _outhit)) (.ImpactPoint (Collision|BreakHitResult _outhit)) 1e+02 (Utilities|Array|MakeArray "ObjectTypeQuery1" "ObjectTypeQuery2") false _array "None"))
    (if _returnvalue_5
      (Transformation|SetActorLocation (Variables|Default|GetBuildingMesh) (.ImpactPoint (Collision|BreakHitResult _outhit)) false false)
      (if (!= (Variables|Default|GetTargetActor) (.HitActor (Collision|BreakHitResult _outhit_2)))
        (bind _output_get (Variables|Default|SetTargetActor (.HitActor (Collision|BreakHitResult _outhit_2))))
        (CallFunction|FindSockets (Actor|GetComponentbyClass _output_get "/Script/Engine.StaticMeshComponent") (Variables|Default|GetSocket%20Location))
        (else
          (bind _array_element (Utilities|Array|ForEachLoopwithBreak (Variables|Default|GetSocket%20Location) :!label _label)
            (:LoopBody
              (if (< (Math|Vector|Distance(Vector) (.ImpactPoint (Collision|BreakHitResult _outhit)) _array_element) 8e+01)
                (Transformation|SetActorLocation (Variables|Default|GetBuildingMesh) _array_element false false)
                (goto _label Break))))))
      (else
        (Variables|Default|SetTargetActor 0)))
    (else
      (Variables|Default|SetTargetActor 0))))

(event EventBeginPlay
  (bind _returnvalue (Game|SpawnActorfromClass "/Game/Blueprints/NewBlueprint.NewBlueprint_C" (Math|Transform|MakeTransform "0, 0, 0" "0, 0, 0" "1.000000,1.000000,1.000000") "AdjustIfPossibleButDontSpawnIfColliding" "MultiplyWithRoot" 0 0))
  (bind _output_get (Variables|Default|SetBuildingMesh _returnvalue))
  (Rendering|SetActorHiddenInGame _output_get false)
  (Components|StaticMesh|SetStaticMesh (Variables|/Script/Engine.StaticMeshActor|GetStaticMeshComponent (Variables|Default|GetBuildingMesh)) "/Game/LevelPrototyping/Meshes/SM_Cube1.SM_Cube1")
  (Rendering|Material|SetOverlayMaterial (Variables|/Script/Engine.StaticMeshActor|GetStaticMeshComponent (Variables|Default|GetBuildingMesh)) "/Game/Material/M_BuildingPreview.M_BuildingPreview" :!class /Script/Engine.MeshComponent))

(event Input|MouseEvents|DebugKeyLeftMouseButton
  (params (Key :type Key%20Structure :default "None") (ActionValue :type Input%20Action%20Value%20Structure))
  (bind _buildingmesh (Variables|Default|GetBuildingMesh))
  (:Pressed
    (Game|SpawnActorfromClass "/Game/Material/Bp_Building.Bp_Building_C" (Math|Transform|MakeTransform (Transformation|GetActorLocation _buildingmesh) (Transformation|GetActorRotation _buildingmesh) "1.000000,1.000000,1.000000") "AdjustIfPossibleButAlwaysSpawn" "MultiplyWithRoot" 0 (Variables|/Script/Engine.StaticMeshComponent|GetStaticMesh (Variables|/Script/Engine.StaticMeshActor|GetStaticMeshComponent (Variables|Default|GetBuildingMesh))) 4.0 0)
    (Transformation|SetActorRotation _buildingmesh)))

(event Input|KeyboardEvents|DebugKeyE
  (params (Key :type Key%20Structure :default "None") (ActionValue :type Input%20Action%20Value%20Structure))
  (:Pressed
    (Transformation|AddWorldRotation (Variables|/Script/Engine.StaticMeshActor|GetStaticMeshComponent (Variables|Default|GetBuildingMesh)) (Math|Rotator|MakeRotator 0.0 0.0 5.0) false false)))

(fn ConstructionScript)