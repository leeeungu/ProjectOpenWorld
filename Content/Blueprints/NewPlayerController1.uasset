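; A player controller that detects the actor the player is looking at and looks up sockets on its static mesh component.
; Each tick, a complex line trace runs from the camera along its view, ignoring the controlled pawn.
; A hit seeds a debug-drawn sphere trace at the impact point to pick a nearby actor.
; Sockets are searched only when that actor changes, and a line trace miss clears the stored actor.
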(event `self.ReceiveTick`
  (params (DeltaSeconds :type "Float (single-precision)"))
  (bind _returnvalue (`GameplayStatics.GetPlayerCameraManager` 0))
  (bind _returnvalue_2 (`PlayerCameraManager.GetCameraLocation` _returnvalue))
  (bind _array (`|MakeArray` (`self.K2_GetPawn`) :!type "Actor Object Reference"))
  (bind (_outhit _returnvalue_3) (`KismetSystemLibrary.LineTraceSingleForObjects` _returnvalue_2 (+ _returnvalue_2 (* (`KismetMathLibrary.GetForwardVector` (`PlayerCameraManager.GetCameraRotation` _returnvalue)) 1200.0)) (`|MakeArray` "ObjectTypeQuery1" "ObjectTypeQuery2" "ObjectTypeQuery4" :!type "EObjectTypeQuery Enum") true _array))
  (if _returnvalue_3
    (bind (_bblockinghit _binitialoverlap _time _distance _location _impactpoint) (`GameplayStatics.BreakHitResult` _outhit))
    (bind (_outhit_2 _returnvalue_4) (`KismetSystemLibrary.SphereTraceSingleForObjects` _impactpoint _impactpoint 100.0 (`|MakeArray` "ObjectTypeQuery1" "ObjectTypeQuery2" :!type "EObjectTypeQuery Enum") false _array "ForDuration"))
    (if _returnvalue_4
      (bind (_bblockinghit_2 _binitialoverlap_2 _time_2 _distance_2 _location_2 _impactpoint_2 _normal _impactnormal _physmat _hitactor) (`GameplayStatics.BreakHitResult` _outhit_2))
      (if (!= (`self.NewVar`) _hitactor)
        (bind _output_get (set `self.NewVar` _hitactor))
        (`/Game/ThirdPerson/Blueprints/FL_Building.FindSockets` (`self.GetComponentByClass` _output_get "/Script/Engine.StaticMeshComponent") (`self.Socket Location`))))
    (else
      (set `self.NewVar` null))))

(fn `UserConstructionScript`)