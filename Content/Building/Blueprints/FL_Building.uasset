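; FL_Building is a building function library with a helper that locates craft sockets on a mesh component.
; FindSockets clears the SocketLocation array, then fills it with the location of every socket whose name contains "Craft".
; It returns false when the mesh component is invalid and true otherwise, even if no socket matches.
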(fn `FindSockets`
  (params (MeshComponent :type "StaticMeshComponent Object Reference (by ref)") (SocketLocation :type "Array of Vector Structure"))
  (returns (SocketResult :type Boolean))
  (`/Engine/EditorBlueprintResources/StandardMacros.IsValid` MeshComponent
    (:`Is Valid`
      (`KismetArrayLibrary.Array_Clear` SocketLocation)
      (for _array_element (`SceneComponent.GetAllSocketNames` MeshComponent)
        (if (`KismetStringLibrary.Contains` (`KismetStringLibrary.Conv_NameToString` _array_element) "Craft")
          (`KismetArrayLibrary.Array_Add` SocketLocation (`SceneComponent.GetSocketLocation` MeshComponent _array_element))))
      (return true))
    (:`Is Not Valid`
      (return false))))