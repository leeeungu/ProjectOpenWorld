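; A test actor that checks whether its static mesh overlaps other geometry and reports what it hits.
; On BeginPlay it teleports to a hard-coded location.
; Every Tick it runs a stationary complex box trace on the Visibility channel, sized from the mesh asset's bounding box and ignoring itself, then prints the hit actor's name.
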(event `self.ReceiveBeginPlay`
  (`self.K2_SetActorLocation` (-5650.0 100.0 500.0) false true))

(event `self.ReceiveTick`
  (params (DeltaSeconds :type "Float (single-precision)"))
  (bind _returnvalue (`self.K2_GetActorLocation`))
  (bind (_outhit _returnvalue_2) (`KismetSystemLibrary.BoxTraceSingle` _returnvalue _returnvalue (* (`KismetMathLibrary.GetBoxSize` (`StaticMesh.GetBoundingBox` (`StaticMeshComponent.StaticMesh` (`self.StaticMesh`)))) 0.5) (struct) "TraceTypeQuery1" true (`|MakeArray` self :!type "Actor Object Reference")))
  (if _returnvalue_2
    (`KismetSystemLibrary.PrintString` (`KismetStringLibrary.Concat_StrStr` (`KismetSystemLibrary.GetDisplayName` (`.HitActor` (`GameplayStatics.BreakHitResult` _outhit))) "Hitted"))))

(fn `UserConstructionScript`)