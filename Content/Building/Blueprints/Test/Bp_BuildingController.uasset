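; Test controller for the building system that drives a BuildingAssistComponent on the possessed pawn through debug key bindings.
; On possess, it finds that component on the pawn or adds one if missing, and caches it.
; Mouse wheel rotates the building in fixed steps, left click spawns it, and right click alternates between starting and ending building through a FlipFlop.
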(event EventPossess
  (params (PossessedPawn :type Pawn%20Object%20Reference))
  (Utilities|IsValid PossessedPawn
    (:Is%20Valid
      (bind _output_get (Variables|Default|SetBuilding%20Assist (Actor|GetComponentbyClass PossessedPawn "/Script/ProjectOpenWorld.BuildingAssistComponent")))
      (Utilities|IsValid _output_get
        (:Is%20Not%20Valid
          (bind _returnvalue (Game|AddComponentbyClass PossessedPawn "/Script/ProjectOpenWorld.BuildingAssistComponent"))
          (Variables|Default|SetBuilding%20Assist _returnvalue))))))

(event Input|MouseEvents|DebugKeyLeftMouseButton
  (params (Key :type Key%20Structure :default "None") (ActionValue :type Input%20Action%20Value%20Structure))
  (:Pressed
    (Class|BuildingAssistComponent|SpawnBuilding (Variables|Default|GetBuilding%20Assist))))

(event Input|MouseEvents|DebugKeyMouseWheelDown
  (params (Key :type Key%20Structure :default "None") (ActionValue :type Input%20Action%20Value%20Structure))
  (:Pressed
    (Class|BuildingAssistComponent|RotateBuilding (Variables|Default|GetBuilding%20Assist) 5.0)))

(event Input|MouseEvents|DebugKeyRightMouseButton
  (params (Key :type Key%20Structure :default "None") (ActionValue :type Input%20Action%20Value%20Structure))
  (:Pressed
    (Utilities|FlowControl|FlipFlop
      (:A
        (Class|BuildingAssistComponent|StartBuilding (Variables|Default|GetBuilding%20Assist)))
      (:B
        (Class|BuildingAssistComponent|EndBuilding (Variables|Default|GetBuilding%20Assist))))))

(event Input|MouseEvents|DebugKeyMouseWheelUp
  (params (Key :type Key%20Structure :default "None") (ActionValue :type Input%20Action%20Value%20Structure))
  (:Pressed
    (Class|BuildingAssistComponent|RotateBuilding (Variables|Default|GetBuilding%20Assist) -5.0)))

(fn ConstructionScript)