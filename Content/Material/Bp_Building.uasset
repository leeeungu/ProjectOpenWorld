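; Building actor that plays a timed construction-progress effect on a configurable static mesh through an overlay material.
; The construction script assigns the mesh, creates a dynamic M_Building overlay and passes it height parameters derived from the mesh bounds and actor location.
; Tick raises FillPercent from its current value to full at a rate set by Timer, then clears the overlay.
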(event `self.ReceiveTick`
  (params (DeltaSeconds :type "Float (single-precision)"))
  (bind _output_get (set `self.Value` (`KismetMathLibrary.FClamp` (+ (`self.Value`) (/ DeltaSeconds (`self.Timer`))))))
  (bind _target (`self.Target`)
    (:`then`
      (`MaterialInstanceDynamic.SetScalarParameterValue` _target "FillPercent" _output_get)
      (if (>= _output_get 1.0)
        (`MeshComponent.SetOverlayMaterial` (`self.StaticMeshComponent`) null)))
    (:`else`)))

(fn `UserConstructionScript`
  (bind (_returnvalue_x _returnvalue_y _returnvalue_z) (`KismetMathLibrary.BreakVector` (`self.K2_GetActorLocation`)))
  (bind _returnvalue (`StaticMesh.GetBoundingBox` (`self.New Mesh`)))
  (`|ExecutionSequence`
    (:`then_0`
      (bind _returnvalue_2 (`KismetMaterialLibrary.CreateDynamicMaterialInstance` "/Game/Material/M_Building.M_Building"))
      (`MeshComponent.SetOverlayMaterial` (`self.StaticMeshComponent`) _returnvalue_2)
      (set `self.Target` _returnvalue_2))
    (:`then_1`
      (bind _target (`self.Target`)
        (:`then`
          (`MaterialInstanceDynamic.SetScalarParameterValue` _target "MeshHeight" (`KismetMathLibrary.Abs` (- (.z (`.Max` (break `Box` _returnvalue))) (.z (break `Box` _returnvalue)))))
          (`MaterialInstanceDynamic.SetScalarParameterValue` _target "MeshWorldHeight" (- _returnvalue_z (.z (break `Box` _returnvalue)))))
        (:`else`)))
    (:`then_2`
      (`StaticMeshComponent.SetStaticMesh` (`self.StaticMeshComponent`) (`self.New Mesh`)))))