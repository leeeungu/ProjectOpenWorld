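; Test player pawn for map testing, with debug keys that toggle climb and travel and command nearby creatures to start or stop building or attacking.
; Sphere traces around the player pick the target: a building actor, or a pawn lacking CreatureMessageInterface.
; A second pawn trace relays the order and target through that interface, looping over hits for building but stopping after one creature for attack.
; All traces draw timed debug shapes.
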(event Custom|CreatureAttackAction
  (params (MessageType :type EMessageType%20Enum :default "NONE"))
  (bind _returnvalue (Transformation|GetActorLocation))
  (bind _returnvalue_2 (Transformation|GetActorLocation))
  (bind _array (Utilities|Array|MakeArray "ObjectTypeQuery3"))
  (bind _self self)
  (bind _array_2 (Utilities|Array|MakeArray _self))
  (bind (_outhits _returnvalue_3) (Collision|MultiSphereTraceForObjects _returnvalue _returnvalue 6e+02 _array false _array_2 "ForDuration" true "(R=0.000000,G=0.096796,B=1.000000,A=1.000000)" "(R=1.000000,G=0.065008,B=0.000000,A=1.000000)" 2.0))
  (if _returnvalue_3
    (bind _array_element (Utilities|Array|ForEachLoopwithBreak _outhits :!label _label)
      (:LoopBody
        (Utilities|Casting|CastToCreatureMessageInterface (.HitActor (Collision|BreakHitResult _array_element))
          (:CastFailed
            (bind (_outhits_2 _returnvalue_4) (Collision|MultiSphereTraceForObjects _returnvalue_2 _returnvalue_2 6e+02 _array false _array_2 "ForDuration" true "(R=1.000000,G=0.000000,B=0.000000,A=1.000000)" "(R=0.000000,G=1.000000,B=0.000000,A=1.000000)" 2.0))
            (if _returnvalue_4
              (for _array_element_2 _outhits_2
                (bind _ascreature_message_interface (Utilities|Casting|CastToCreatureMessageInterface (.HitActor (Collision|BreakHitResult _array_element_2))))
                (Class|CreatureMessageInterface|ReceiveMessage _ascreature_message_interface MessageType self (.HitActor (Collision|BreakHitResult _array_element)))
                (goto _label Break))
              (goto _label Break))))))))

(event Custom|CreatureBuildingAction
  (params (MessageType :type EMessageType%20Enum :default "NONE"))
  (bind _returnvalue (Transformation|GetActorLocation))
  (bind _returnvalue_2 (Transformation|GetActorLocation))
  (bind _self self)
  (bind _array (Utilities|Array|MakeArray _self))
  (bind (_outhit _returnvalue_3) (Collision|SphereTraceForObjects _returnvalue_2 _returnvalue_2 6e+02 (Utilities|Array|MakeArray "ObjectTypeQuery2" "ObjectTypeQuery1") true _array "ForDuration" true "(R=0.000000,G=0.103947,B=1.000000,A=1.000000)" "(R=0.000000,G=1.000000,B=0.000000,A=1.000000)" 2.0))
  (if _returnvalue_3
    (bind _asbp_building_actor (Utilities|Casting|CastToBp_BuildingActor (.HitActor (Collision|BreakHitResult _outhit))))
    (bind (_outhits _returnvalue_4) (Collision|MultiSphereTraceForObjects _returnvalue _returnvalue 6e+02 (Utilities|Array|MakeArray "ObjectTypeQuery3") false _array "ForDuration" true "(R=1.000000,G=0.000000,B=0.000000,A=1.000000)" "(R=0.000000,G=1.000000,B=0.000000,A=1.000000)" 2.0))
    (if _returnvalue_4
      (for _array_element _outhits
        (bind _ascreature_message_interface (Utilities|Casting|CastToCreatureMessageInterface (.HitActor (Collision|BreakHitResult _array_element))))
        (Class|CreatureMessageInterface|ReceiveMessage _ascreature_message_interface MessageType self _asbp_building_actor)))))

(event Input|KeyboardEvents|DebugKeyF
  (params (Key :type Key%20Structure) (ActionValue :type Input%20Action%20Value%20Structure))
  (:Pressed
    (Utilities|FlowControl|FlipFlop
      (:A
        (Class|BasePlayer|StartClimb))
      (:B
        (Class|BasePlayer|StartTravel)))))

(event Input|KeyboardEvents|DebugKeyG
  (params (Key :type Key%20Structure) (ActionValue :type Input%20Action%20Value%20Structure))
  (:Pressed
    (CallFunction|CreatureBuildingAction "DoBuild")))

(event Input|KeyboardEvents|DebugKeyH
  (params (Key :type Key%20Structure) (ActionValue :type Input%20Action%20Value%20Structure))
  (:Pressed
    (CallFunction|CreatureBuildingAction "StopBuild")))

(event Input|KeyboardEvents|DebugKey1
  (params (Key :type Key%20Structure) (ActionValue :type Input%20Action%20Value%20Structure))
  (:Pressed
    (CallFunction|CreatureAttackAction "DoAttack")))

(event Input|KeyboardEvents|DebugKey2
  (params (Key :type Key%20Structure) (ActionValue :type Input%20Action%20Value%20Structure))
  (:Pressed
    (CallFunction|CreatureAttackAction "StopAttack")))

(fn ConstructionScript)