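; Test monster actor, apparently a target for checking damage handling.
; AnyDamage adds incoming damage to a running total, prints it, and destroys the actor once the total reaches a fixed threshold.
; A separate DamagedCharacter function only prints the other object's attack value and returns false, without touching that total.
; BeginPlay, overlap, Tick and the construction script are empty.
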(event `self.ReceiveAnyDamage`
  (params (Damage :type "Float (single-precision)") (DamageType :type "DamageType Object Reference") (InstigatedBy :type "Controller Object Reference") (DamageCauser :type "Actor Object Reference"))
  (bind _output_get (set `self.NewVar` (+ Damage (`self.NewVar`))))
  (`KismetSystemLibrary.PrintString` (`KismetStringLibrary.Conv_DoubleToString` _output_get))
  (if (>= (`self.NewVar`) 100.0)
    (`self.K2_DestroyActor`)))

(fn `DamagedCharacter`
  (params (Other :type "AttackInterface Interface (by ref)"))
  (returns (ReturnValue :type Boolean))
  (`KismetSystemLibrary.PrintString` (`KismetStringLibrary.Conv_DoubleToString` (`AttackInterface.GetAttackValue` Other)))
  (return false))

(fn `UserConstructionScript`)