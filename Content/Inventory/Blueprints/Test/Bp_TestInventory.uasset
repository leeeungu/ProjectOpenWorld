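; Test Blueprint in the Inventory test folder for manually driving animation sections on the player's animation Blueprint.
; Three debug keys each cast the mesh's anim instance to ABP_Player.
; The first key starts an anim section, the second ends it, and the third prints the current section type.
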(event Input|KeyboardEvents|DebugKey3
  (params (Key :type Key%20Structure :default "None") (ActionValue :type Input%20Action%20Value%20Structure))
  (:Pressed
    (bind _asabp_player (Utilities|Casting|CastToABP_Player (Components|SkeletalMesh|GetAnimInstance (Variables|Character|GetMesh))))
    (Development|PrintString (Utilities|String|EnumtoString (Class|PlayerAnimInstance|GetAnimSectionType _asabp_player)))))

(event Input|KeyboardEvents|DebugKey1
  (params (Key :type Key%20Structure :default "None") (ActionValue :type Input%20Action%20Value%20Structure))
  (:Pressed
    (bind _asabp_player (Utilities|Casting|CastToABP_Player (Components|SkeletalMesh|GetAnimInstance (Variables|Character|GetMesh))))
    (Class|PlayerAnimInstance|StartAnimSection _asabp_player)))

(event Input|KeyboardEvents|DebugKey2
  (params (Key :type Key%20Structure :default "None") (ActionValue :type Input%20Action%20Value%20Structure))
  (:Pressed
    (bind _asabp_player (Utilities|Casting|CastToABP_Player (Components|SkeletalMesh|GetAnimInstance (Variables|Character|GetMesh))))
    (Class|PlayerAnimInstance|EndAnimSection _asabp_player)))

(fn ConstructionScript)