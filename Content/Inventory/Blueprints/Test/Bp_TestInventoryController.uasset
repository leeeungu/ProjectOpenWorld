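; Test controller for the inventory system that seeds its InventoryComponent with starter items at BeginPlay.
; After the parent BeginPlay, a sequence creates BaseItem instances for a steel pickaxe, a sword and a steel axe, then adds each to the component.
; Older ID-and-count AddItem calls for other items, including resources, remain in the graph but are disconnected.
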(event `self.ReceiveBeginPlay`
  (`parent.ReceiveBeginPlay`)
  (`|ExecutionSequence`
    (:`then_0`
      (bind _returnvalue (`ItemFunctionLibrary.CreateBaseItem` "Pickaxe_Steal" 1 self "/Script/ProjectOpenWorld.BaseItem"))
      (`InventoryComponent.AddItem` (`self.InventoryComponent`) _returnvalue))
    (:`then_1`
      (bind _returnvalue_2 (`ItemFunctionLibrary.CreateBaseItem` "Sword" 1 self "/Script/ProjectOpenWorld.BaseItem"))
      (`InventoryComponent.AddItem` (`self.InventoryComponent`) _returnvalue_2))
    (:`then_2`
      (bind _returnvalue_3 (`ItemFunctionLibrary.CreateBaseItem` "Axe_Steal" 1 self "/Script/ProjectOpenWorld.BaseItem"))
      (`InventoryComponent.AddItem` (`self.InventoryComponent`) _returnvalue_3))))

(fn `UserConstructionScript`)